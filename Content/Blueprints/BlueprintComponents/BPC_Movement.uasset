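; Player movement component that handles crouching, sprinting and stamina by changing the character's max walk speed.
; Crouch events also have L1_Character shorten or lengthen its capsule.
; SprintHeld drains stamina by frame delta while the player moves uncrouched, stopping at minimum.
; StopSprint restores walk speed, then after a delay starts a looping timer to refill stamina, which sprinting cancels; StartSprint is deprecated.
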(event Custom|StartSprint
  ;[1 1 1] deprecated
  (if (and (> (Variables|Default|GetCurrentStamina) (Variables|Default|GetMinStamina)) (not (Variables|Default|GetisCrouching)))
    (Utilities|Time|ClearandInvalidateTimerbyHandle (Variables|Default|GetStaminaHandler))
    (CallFunction|SetPlayerMaxWalkSpeed (Variables|Default|GetSprintSpeed))))

(event Custom|SprintHeld
  (bind _staminahandler (Variables|Default|GetStaminaHandler))
  ;[1 1 1] SPRINT AND STAMINA
  ;;[1 1 1] Checks for sprint conditions every frame when holding Sprint, then calls Decrease Stamina
  (if (> (Math|Vector|VectorLength (Transformation|GetVelocity (Variables|Default|GetPlayer%20Ref))) 1e+01)
    (if (not (Variables|Default|GetisCrouching))
      (Utilities|FlowControl|Sequence
        (:then_0
          (CallFunction|DecreaseStamina))
        (:then_1
          (if (Utilities|Time|IsTimerActivebyHandle _staminahandler)
            (Utilities|Time|ClearandInvalidateTimerbyHandle _staminahandler)))))
    (elif (not (Utilities|Time|IsTimerActivebyHandle (Variables|Default|GetStaminaHandler)))
      (CallFunction|StopSprint))))

(event Custom|StopSprint
  ;[1 1 1] SPRINT AND STAMINA
  ;;[1 1 1] Stops sprinting and sets us at walking speed; when IA_Sprint is released, delays then starts Stamina Recovery Timer
  (CallFunction|SetPlayerMaxWalkSpeed (Variables|Default|GetWalkSpeed))
  (Utilities|FlowControl|Delay 3.0)
  (bind _returnvalue (Utilities|Time|SetTimerbyEvent (EventDispatchers|CreateEvent :!event Custom|SprintRecoveryTimer) 0.05 true))
  (Variables|Default|SetStaminaHandler _returnvalue))

(event Custom|SprintRecoveryTimer
  ;[1 1 1] SPRINT AND STAMINA
  ;;[1 1 1] Recovers stamina up to Max while IA_Sprint is NOT pressed, then invalidates stamina timer
  (Variables|Default|SetCurrentStamina (Math|Float|Clamp(Float) (+ (Variables|Default|GetCurrentStamina) 1.0) (Variables|Default|GetMinStamina) (Variables|Default|GetMaxStamina)))
  (if (>= (Variables|Default|GetCurrentStamina) (Variables|Default|GetMaxStamina))
    (Utilities|Time|ClearandInvalidateTimerbyHandle (Variables|Default|GetStaminaHandler))))

(event Custom|DecreaseStamina
  ;[1 1 1] SPRINT AND STAMINA
  ;;[1 1 1] Sets sprint speed and decreases stamina while we are sprinting until stamina is at Min; then calls Stop Sprint
  (CallFunction|SetPlayerMaxWalkSpeed (Variables|Default|GetSprintSpeed))
  (if (> (Math|Vector|VectorLength (Transformation|GetVelocity (Variables|Default|GetPlayer%20Ref))) 1e+01)
    (Variables|Default|SetCurrentStamina (Math|Float|Clamp(Float) (- (Variables|Default|GetCurrentStamina) (* (Utilities|Time|GetWorldDeltaSeconds) (Variables|Default|GetStaminaDecreaseRate))) (Variables|Default|GetMinStamina) (Variables|Default|GetMaxStamina)))
    (if (<= (Variables|Default|GetCurrentStamina) (Variables|Default|GetMinStamina))
      (CallFunction|StopSprint))
    (else
      (CallFunction|StopSprint))))

(event Custom|StartCrouch
  ;[1 1 1] Crouch
  (Default|ShortenPlayerCapsule (.AsL1%20Character (Utilities|Casting|CastToL1_Character (Variables|Default|GetPlayer%20Ref))))
  (Variables|Default|SetisCrouching true)
  (CallFunction|SetPlayerMaxWalkSpeed (Variables|Default|GetCrouchSpeed)))

(event Custom|EndCrouch
  ;[1 1 1] Crouch
  (Default|LengthenPlayerCapsule (.AsL1%20Character (Utilities|Casting|CastToL1_Character (Variables|Default|GetPlayer%20Ref))))
  (Variables|Default|SetisCrouching false)
  (CallFunction|SetPlayerMaxWalkSpeed (Variables|Default|GetWalkSpeed)))

(fn Initialise
  (params (Character :type Character%20Object%20Reference))
  (Variables|Default|SetPlayer%20Ref Character)
  (Variables|/Script/Engine.CharacterMovementComponent|SetMaxWalkSpeed (Variables|/Script/Engine.Character|GetCharacterMovement (Variables|Default|GetPlayer%20Ref)) (Variables|Default|GetWalkSpeed))
  (Variables|Default|SetCrouchHalfHeight (Variables|Default|GetCrouchHalfHeight)))

(fn SetPlayerMaxWalkSpeed
  (params (MaxWalkSpeed :type Float%20%28single-precision%29))
  (Variables|/Script/Engine.CharacterMovementComponent|SetMaxWalkSpeed (Variables|/Script/Engine.Character|GetCharacterMovement (Variables|Default|GetPlayer%20Ref)) MaxWalkSpeed))
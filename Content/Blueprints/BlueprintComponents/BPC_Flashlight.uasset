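; Flashlight component that gives the player a toggleable light with limited battery life.
; Initialise stores the player reference and grabs its Flashlight light, which ToggleFlashlight shows only if charge is above the minimum.
; While lit, a looping function-name timer drains the clamped battery level, switching the light off and clearing itself at the minimum.
; AddBatteryLife restores charge within the same limits.
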(event EventBeginPlay)

(event EventTick
  (params (DeltaSeconds :type Float%20%28single-precision%29)))

(fn ToggleFlashlight
  (bind _flashlightlight (Variables|Default|GetFlashlightLight))
  (if (Variables|/Script/Engine.SceneComponent|GetbVisible _flashlightlight)
    (Rendering|SetVisibility _flashlightlight false false)
    (Utilities|Time|ClearTimerbyFunctionName 0 "DepleteBatteryLife")
    (elif (> (Variables|Default|GetCurrentBatteryLevel) (Variables|Default|GetMinBatteryLevel))
      (Rendering|SetVisibility _flashlightlight true false)
      (Utilities|Time|SetTimerbyFunctionName 0 "DepleteBatteryLife" (Variables|Default|GetBatteryDecreaseRate) true))))

(fn Initialise
  (params (Player :type L1%20Character%20Object%20Reference))
  (bind _output_get (Variables|Default|SetPlayerRef Player))
  (Variables|Default|SetFlashlightLight (Variables|/Game/GameBP/Level1/L1_Character.L1_Character_C|GetFlashlight _output_get)))

(fn DepleteBatteryLife
  (bind _output_get (Variables|Default|SetCurrentBatteryLevel (Math|Float|Clamp(Float) (- (Variables|Default|GetCurrentBatteryLevel) (Variables|Default|GetDepletionAmount)) (Variables|Default|GetMinBatteryLevel) (Variables|Default|GetMaxBatteryLevel))))
  (if (<= _output_get (Variables|Default|GetMinBatteryLevel))
    (Rendering|SetVisibility (Variables|Default|GetFlashlightLight) false false)
    (Utilities|Time|ClearTimerbyFunctionName 0 "DepleteBatteryLife")))

(fn AddBatteryLife
  (params (Amount :type Float%20%28double-precision%29))
  (Variables|Default|SetCurrentBatteryLevel (Math|Float|Clamp(Float) (+ Amount (Variables|Default|GetCurrentBatteryLevel)) (Variables|Default|GetMinBatteryLevel) (Variables|Default|GetMaxBatteryLevel))))
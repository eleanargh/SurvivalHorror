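; Inventory component that holds the player's items as a slot array sized from HG_PlayerController and refreshes the matching grid widget slots as contents change.
; AddItem fills partial stacks, then empty slots, recursing on overflow and returning any remainder.
; UseItem calls UseItem on an existing or spawned item actor, removing one on success, while DropItem spawns a physics pickup ahead of the player.
; It also supports adding slots and finding or removing items by tag.
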(event Custom|Initialize
  (bind _returnvalue (Game|GetPlayerController 0))
  (bind _ashg_player_controller (Utilities|Casting|CastToHG_PlayerController _returnvalue))
  ;[1 1 1] On begin play, set inventory slots array length as the length of inventory slots in game
  (Utilities|Array|Resize (Variables|Default|GetInventorySlots) (Variables|/Game/GameBP/HG_PlayerController.HG_PlayerController_C|GetInventorySlots _ashg_player_controller))
  (Variables|Default|SetW%20Inventory%20Menu%20Ref (Variables|/Game/GameBP/HG_PlayerController.HG_PlayerController_C|GetW_InventoryMenuRef _ashg_player_controller))
  (bind _asl1_character (Utilities|Casting|CastToL1_Character (Game|GetPlayerCharacter 0)))
  (Variables|Default|SetPlayerRef _asl1_character))

(event EventBeginPlay
  (CallFunction|Initialize))

(fn AddItem
  (params (Item :type BP%20Inventory%20Item%20Master%20Class%20Reference) (Amount :type Integer))
  (bind (_success_ _index) (CallFunction|CheckforEmptySlot))
  (bind (_success__2 _index_2) (CallFunction|CheckforEmptySlot))
  (LocalVariables|SetLocalItem Item)
  (LocalVariables|SetLocalAmount Amount)
  ;[1 1 1] Is it possible to have a stack of this item?
  (LocalVariables|SetLocalMaxStackAmount (.MaxStackAmount (Utilities|Struct|BreakS_ItemData (.ItemData (Utilities|GetClassDefaults (LocalVariables|GetLocalItem))))))
  (if (> (.MaxStackAmount (Utilities|Struct|BreakS_ItemData (.ItemData (Utilities|GetClassDefaults (LocalVariables|GetLocalItem))))) 1)
    ;[1 1 1] Do we have an existing stack? If so, return the index of that slot.
    (bind (_success__3 _index_3) (CallFunction|CheckforSlotwithSpace (LocalVariables|GetLocalItem)))
    (if _success__3
      (LocalVariables|SetLocalIndex _index_3)
      ;[1 1 1] Is the amount of item greater than the max stack we can have in this slot?
      (if (> (+ (.Amount (CallFunction|GetItemDataatIndex (LocalVariables|GetLocalIndex))) (LocalVariables|GetLocalAmount)) (LocalVariables|GetLocalMaxStackAmount))
        (LocalVariables|SetLocalAmount (- (+ (.Amount (CallFunction|GetItemDataatIndex (LocalVariables|GetLocalIndex))) (LocalVariables|GetLocalAmount)) (LocalVariables|GetLocalMaxStackAmount)))
        ;[1 1 1] Put a full stack in the free inventory slot, then run Add Item again to check what we do with the remainder.
        (Utilities|Array|SetArrayElem (Variables|Default|GetInventorySlots) (LocalVariables|GetLocalIndex) (Utilities|Struct|MakeS_InventoryItems (LocalVariables|GetLocalItem) (LocalVariables|GetLocalMaxStackAmount)) :!label _label)
        (CallFunction|UpdateInventorySlot (LocalVariables|GetLocalIndex))
        (bind _remainder (CallFunction|AddItem (LocalVariables|GetLocalItem) (- (LocalVariables|GetLocalAmount) (LocalVariables|GetLocalMaxStackAmount))))
        (return true _remainder)
        (else
          (Utilities|Array|SetArrayElem (Variables|Default|GetInventorySlots) (LocalVariables|GetLocalIndex) (Utilities|Struct|MakeS_InventoryItems (LocalVariables|GetLocalItem) (+ (.Amount (CallFunction|GetItemDataatIndex (LocalVariables|GetLocalIndex))) (LocalVariables|GetLocalAmount))))
          ;[1 1 1] Update the inventory widget
          (CallFunction|UpdateInventorySlot (LocalVariables|GetLocalIndex))
          (return true 0)))
      (else
        ;[1 1 1] Do we have an empty slot?
        (if _success__2
          (LocalVariables|SetLocalIndex _index_2)
          ;[1 1 1] Is the amount being picked up larger than a single stack?
          (if (> (LocalVariables|GetLocalAmount) (LocalVariables|GetLocalMaxStackAmount))
            (goto _label)
            (else
              (Utilities|Array|SetArrayElem (Variables|Default|GetInventorySlots) (LocalVariables|GetLocalIndex) (Utilities|Struct|MakeS_InventoryItems (LocalVariables|GetLocalItem) (LocalVariables|GetLocalAmount)))
              (CallFunction|UpdateInventorySlot (LocalVariables|GetLocalIndex))
              (return true 0)))
          (else
            _))))
    (else
      ;[1 1 1] Did we find an empty slot? If so, return index of empty slot.
      (if _success_
        (bind _output_get (LocalVariables|SetLocalIndex _index))
        ;[1 1 1] Add the item and amount to the inventory array at the index returned.
        (Utilities|Array|SetArrayElem (Variables|Default|GetInventorySlots) _output_get (Utilities|Struct|MakeS_InventoryItems (LocalVariables|GetLocalItem) 1))
        ;[1 1 1] Update the inventory widget
        (CallFunction|UpdateInventorySlot (LocalVariables|GetLocalIndex))
        (if (> (- (LocalVariables|GetLocalAmount) 1) 0)
          (bind _remainder_2 (CallFunction|AddItem (LocalVariables|GetLocalItem) (- (LocalVariables|GetLocalAmount) 1)))
          (return true _remainder_2)
          (else
            (return true 0)))
        (else
          _))))
  (Development|PrintString "no free slots :(")
  (return false (LocalVariables|GetLocalAmount)))

(fn CheckforEmptySlot
  ;[1 1 1] For each slot in the inventory array, check to see if the item in it is valid. If it is, keep going through the loop until an empty slot is found. If no empty slot found, return success false. If found, return success true and index number of empty slot.
  (bind (_array_element _array_index) (Utilities|Array|ForEachLoopwithBreak (Variables|Default|GetInventorySlots) :!label _label)
    (:LoopBody
      (if (Utilities|IsValidClass (.Item (Utilities|Struct|BreakS_InventoryItems _array_element)))
        (LocalVariables|SetLocalSuccess false)
        (else
          (LocalVariables|SetLocalSuccess true)
          (LocalVariables|SetLocalIndex _array_index)
          (goto _label Break))))
    (:Completed
      (return (LocalVariables|GetLocalSuccess) (LocalVariables|GetLocalIndex)))))

(fn GetItemDataatIndex
  (params (Index :type Integer))
  (bind _inventoryslots (Variables|Default|GetInventorySlots))
  (bind _output (Utilities|Array|Get(acopy) _inventoryslots Index))
  (bind (_item _amount) (Utilities|Struct|BreakS_InventoryItems _output))
  ;[1 1 1] Gets the information about an item in a particular inventory slot
  (return _item _amount))

(fn UpdateInventorySlot
  (params (Index :type Integer))
  ;[1 1 1] Locate the specific inventory slot we're updating, then call update slot.
  (Default|UpdateSlot (Utilities|Array|Get(acopy) (Variables|/Game/UMG/Inventory/W_InventoryGrid.W_InventoryGrid_C|GetSlotsArray (Variables|/Game/UMG/Inventory/W_InventoryMenu.W_InventoryMenu_C|GetW_InventoryGrid (Variables|/Game/GameBP/HG_PlayerController.HG_PlayerController_C|GetW_InventoryMenuRef (.AsHG%20Player%20Controller (Utilities|Casting|CastToHG_PlayerController (Game|GetPlayerController 0)))))) Index)))

(fn CheckforSlotwithSpace
  (params (Item :type BP%20Inventory%20Item%20Master%20Class%20Reference))
  ;[1 1 1] For each slot in the array, check to see if we have the item already and if we are less than the max stack of the item. Return local success false if we aren't and true if we are.
  (bind (_array_element _array_index) (Utilities|Array|ForEachLoopwithBreak (Variables|Default|GetInventorySlots) :!label _label)
    (:LoopBody
      (if (and (== (.Item (Utilities|Struct|BreakS_InventoryItems _array_element)) Item) (< (.Amount (Utilities|Struct|BreakS_InventoryItems _array_element)) (.maxstackamount (.ItemData (Utilities|GetClassDefaults Item)))))
        (LocalVariables|SetLocalSuccess true)
        (LocalVariables|SetLocalIndex _array_index)
        (goto _label Break)
        (else
          (LocalVariables|SetLocalSuccess false))))
    (:Completed
      (return (LocalVariables|GetLocalSuccess) (LocalVariables|GetLocalIndex)))))

(fn UseItem
  (params (Index :type Integer))
  (bind _output_get (LocalVariables|SetLocalIndex Index))
  ;[1 1 1] Calls 'Use item' on the item at the index we are looking at; Use Item is definied in individual item blueprints
  (if (> (.Amount (CallFunction|GetItemDataatIndex _output_get)) 0)
    (bind _returnvalue (Actor|GetActorOfClass (.Item (CallFunction|GetItemDataatIndex _output_get))))
    (Utilities|IsValid _returnvalue
      (:Is%20Valid
        (Default|UseItem _returnvalue)
        (if (Variables|/Game/Blueprints/Actors/Inventory/BP_InventoryItem_Master.BP_InventoryItem_Master_C|GetUseItemSuccess _returnvalue)
          (CallFunction|RemoveItematIndex (LocalVariables|GetLocalIndex) :!label _label)
          (Default|CloseDropDownMenu (Variables|Default|GetW%20Inventory%20Menu%20Ref))
          (else
            (Development|PrintString "use item not successful" :!label _label_2))))
      (:Is%20Not%20Valid
        (bind _returnvalue_2 (Game|SpawnActorfromClass (.Item (CallFunction|GetItemDataatIndex _output_get)) (Math|Transform|MakeTransform "0, 0, 0" "0, 0, 0" "1.000000,1.000000,1.000000") "Undefined" "MultiplyWithRoot" 0 0))
        (Default|UseItem _returnvalue_2)
        (if (Variables|/Game/Blueprints/Actors/Inventory/BP_InventoryItem_Master.BP_InventoryItem_Master_C|GetUseItemSuccess _returnvalue_2)
          (goto _label)
          (else
            (goto _label_2)))))))

(fn RemoveItematIndex
  (params (Index :type Integer))
  (bind (_item _amount) (CallFunction|GetItemDataatIndex Index))
  (bind _inventoryslots (Variables|Default|GetInventorySlots))
  (if (> _amount 1)
    (Utilities|Array|SetArrayElem _inventoryslots Index (Utilities|Struct|MakeS_InventoryItems _item (- _amount 1)))
    (else
      (Utilities|Array|SetArrayElem _inventoryslots Index (Utilities|Struct|MakeS_InventoryItems 0 0))))
  (CallFunction|UpdateInventorySlot Index))

(fn DropItem
  (params (Index :type Integer))
  (bind _playerref (Variables|Default|GetPlayerRef))
  (bind _rootcomponent (Variables|/Script/Engine.Actor|GetRootComponent _playerref))
  (bind _returnvalue (Transformation|GetWorldLocation _rootcomponent))
  ;[0.15 0.15 0.15 0.5] sets the item class + amount being dropped at this index
  (bind _output_get (LocalVariables|SetLocalIndex Index))
  (LocalVariables|SetLocalAmount (.Amount (CallFunction|GetItemDataatIndex _output_get)))
  (LocalVariables|SetLocalClass (.Item (CallFunction|GetItemDataatIndex _output_get)))
  ;[0.15 0.15 0.15 0.5] checks there is more than 0 at this index
  (if (> (LocalVariables|GetLocalAmount) 0)
    ;[0.15 0.15 0.15 0.5] removes entire stack at index (1 at a time??)
    (for _index (range 1 (LocalVariables|GetLocalAmount))
      (CallFunction|RemoveItematIndex (LocalVariables|GetLocalIndex)))
    (Default|CloseDropDownMenu (Variables|Default|GetW%20Inventory%20Menu%20Ref))
    ;[0.15 0.15 0.15 0.5] Draw a line trace between player world loc and 200 ahead
    (bind (_outhit _returnvalue_2) (Collision|LineTraceByChannel _returnvalue (+ _returnvalue (* (Math|Vector|GetForwardVector (Variables|/Script/Engine.Actor|GetRootComponent _playerref)) 2e+02)) "TraceTypeQuery1" false 0 "None"))
    ;[0.15 0.15 0.15 0.5] Spawns the correct pickup actor for inventory item, using local amount as the quantity to spawn (in a stack)
    (bind _returnvalue_3 (Game|SpawnActorfromClass (.pickupactor (.ItemData (Utilities|GetClassDefaults (LocalVariables|GetLocalClass)))) (Math|Transform|MakeTransform (select _returnvalue_2 (.Location (Collision|BreakHitResult _outhit)) (.TraceEnd (Collision|BreakHitResult _outhit))) "0, 0, 0" "1.000000,1.000000,1.000000") "Undefined" "MultiplyWithRoot" 0 0))
    (Variables|/Game/Blueprints/Actors/Inventory/PickupActors/BP_PickupActor_Master.BP_PickupActor_Master_C|SetAmount _returnvalue_3 (LocalVariables|GetLocalAmount))
    (Physics|SetSimulatePhysics (Variables|/Game/Blueprints/Actors/Inventory/PickupActors/BP_PickupActor_Master.BP_PickupActor_Master_C|GetStaticMesh _returnvalue_3) true)))

(fn AddMoreSlots
  (params (Amount :type Integer))
  (bind _returnvalue (Game|GetPlayerController 0))
  (bind _w_inventory_menu_ref (Variables|Default|GetW%20Inventory%20Menu%20Ref))
  (bind _ashg_player_controller (Utilities|Casting|CastToHG_PlayerController _returnvalue))
  (bind _w_inventorygrid (Variables|/Game/UMG/Inventory/W_InventoryMenu.W_InventoryMenu_C|GetW_InventoryGrid _w_inventory_menu_ref))
  ;[0.15 0.15 0.15 0.5] Changes the size of the inventory array to inventory array+amount of slots added by the item calling AddMoreSlots
  (bind _output_get (Variables|/Game/GameBP/HG_PlayerController.HG_PlayerController_C|SetInventorySlots _ashg_player_controller (+ Amount (Variables|/Game/GameBP/HG_PlayerController.HG_PlayerController_C|GetInventorySlots _ashg_player_controller))))
  (Utilities|Array|Resize (Variables|Default|GetInventorySlots) _output_get)
  (Default|AddMoreSlots _w_inventorygrid Amount)
  (for _array_element (Variables|/Game/UMG/Inventory/W_InventoryGrid.W_InventoryGrid_C|GetSlotsArray _w_inventorygrid)
    (Default|Initialise _array_element _w_inventory_menu_ref)))

(fn CheckforItembyTag
  (params (Item%20Tag :type Gameplay%20Tag%20Structure))
  (bind _array_element (Utilities|Array|ForEachLoopwithBreak (Variables|Default|GetInventorySlots) :!label _label)
    (:LoopBody
      (if (GameplayTags|HasTag (.ItemTags (Utilities|GetClassDefaults (.Item (Utilities|Struct|BreakS_InventoryItems _array_element)))) Item%20Tag true)
        (LocalVariables|SetLocalSuccess true)
        (goto _label Break)
        (else
          (LocalVariables|SetLocalSuccess false))))
    (:Completed
      (return (LocalVariables|GetLocalSuccess)))))

(fn RemoveItembyTag
  (params (ItemTag :type Gameplay%20Tag%20Structure))
  (bind (_array_element _array_index) (Utilities|Array|ForEachLoopwithBreak (Variables|Default|GetInventorySlots) :!label _label)
    (:LoopBody
      (if (GameplayTags|HasTag (.ItemTags (Utilities|GetClassDefaults (.Item (Utilities|Struct|BreakS_InventoryItems _array_element)))) ItemTag true)
        (CallFunction|RemoveItematIndex _array_index)
        (goto _label Break)))))
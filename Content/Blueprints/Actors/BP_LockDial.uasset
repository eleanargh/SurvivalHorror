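; BP_LockDial is a lock dial actor that rotates in 36-degree steps and tracks the number it displays.
; A looping one-second timer with randomized start delay calls RotateDial, gated by CanRotate to prevent overlapping turns.
; A timeline lerps the mesh roll through each step, then updates DialRotation, resetting it to zero at 360.
; FindNumber converts that rotation into NumberDisplayed and prints it on BeginPlay and after each turn.
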(event Custom|FindNumber
  ;[0.15 0.15 0.15 0.5] interprets dial rotation as the number displayed (36 degrees between each number)
  (bind _output_get (Variables|Default|SetNumberDisplayed (Math|Float|Truncate (/ (Variables|Default|GetDialRotation) 36.0))))
  (Development|PrintString (Utilities|String|ToString(Integer) _output_get)))

(event Custom|RotateDial
  (if (Variables|Default|GetCanRotate)
    (Variables|Default|SetCanRotate false)
    (bind _alpha (Timeline|RotateDialTL Play)
      (:Update
        (Transformation|SetRelativeRotation (Variables|Default|GetLockDialMesh) (Math|Rotator|MakeRotator (+ (Variables|Default|GetDialRotation) (Math|Float|Lerp 0.0 36.0 _alpha)) 0.0 0.0) false false))
      (:Finished
        ;[0.15 0.15 0.15 0.5] sets the dial rotation back to zero if it goes above 360
        (Variables|Default|SetDialRotation (+ (Variables|Default|GetDialRotation) (Math|Float|Lerp 0.0 36.0 _alpha)))
        (if (>= (Variables|Default|GetDialRotation) 3.6e+02)
          (Variables|Default|SetDialRotation 0.0)
          (Transformation|SetRelativeRotation (Variables|Default|GetLockDialMesh) "0, 0, 0" false false))
        (CallFunction|FindNumber)
        (Variables|Default|SetCanRotate true)))))

(event EventBeginPlay
  (CallFunction|FindNumber)
  (Utilities|Time|SetTimerbyFunctionName 0 "RotateDial" 1.0 true false 0.0 2.0))

(fn ConstructionScript)
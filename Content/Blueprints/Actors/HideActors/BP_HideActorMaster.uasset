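; Base hiding-spot actor that lets the player move into and out of hiding on interact.
; Interact starts a looping timer that glides the player to HidingPosition or ExitPosition, then fires a finished-moving dispatcher and toggles IsHiding.
; Collision, movement and inventory access are disabled on entry and restored after exit.
; Sphere overlap drives a "Hide" button prompt; player rotation exists but is flagged as needing a fix.
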(event OnComponentBeginOverlap(Sphere)
  (params (OverlappedComponent :type Primitive%20Component%20Object%20Reference) (OtherActor :type Actor%20Object%20Reference) (OtherComp :type Primitive%20Component%20Object%20Reference) (OtherBodyIndex :type Integer) (bFromSweep :type Boolean) (SweepResult :type Hit%20Result%20Structure%20%28by%20ref%29))
  ;[0.15 0.15 0.15 0.5] Contextual Prompt
  (Utilities|Casting|CastToL1_Character OtherActor)
  (Rendering|SetVisibility (Variables|Default|GetContextButtonPromptWidget) true false)
  (Variables|Default|SetUpdateActor true)
  (bind _asw_context_button_prompt (Utilities|Casting|CastToW_ContextButtonPrompt (UserInterface|GetUserWidgetObject (Variables|Default|GetContextButtonPromptWidget))))
  (Rendering|Components|TextRender|SetText (Variables|/Game/UMG/W_ContextButtonPrompt.W_ContextButtonPrompt_C|GetButtontext _asw_context_button_prompt) "Hide")
  (bind _asw_context_button_prompt_2 (Utilities|Casting|CastToW_ContextButtonPrompt (UserInterface|GetUserWidgetObject (Variables|Default|GetContextButtonPromptWidget))))
  (Variables|/Script/UMG.TextBlock|SetText (Variables|/Game/UMG/W_ContextButtonPrompt.W_ContextButtonPrompt_C|GetButtonprompt_1 _asw_context_button_prompt_2) "E"))

(event OnComponentEndOverlap(Sphere)
  (params (OverlappedComponent :type Primitive%20Component%20Object%20Reference) (OtherActor :type Actor%20Object%20Reference) (OtherComp :type Primitive%20Component%20Object%20Reference) (OtherBodyIndex :type Integer))
  ;[0.15 0.15 0.15 0.5] Contextual Prompt
  (Utilities|Casting|CastToL1_Character OtherActor)
  (Rendering|SetVisibility (Variables|Default|GetContextButtonPromptWidget) false false)
  (Variables|Default|SetUpdateActor false))

(event Custom|MoveCharacter
  (bind _playerref (Variables|Default|GetPlayerRef))
  (Transformation|SetActorTransform _playerref (Math|Transform|MakeTransform (Math|Interpolation|VInterptoConstant (Transformation|GetActorLocation _playerref) (Transformation|GetWorldLocation (select (Variables|/Game/GameBP/Level1/L1_Character.L1_Character_C|GetIsHiding (Variables|Default|GetPlayerRef)) (Variables|Default|GetExitPosition) (Variables|Default|GetHidingPosition))) (Utilities|Time|GetWorldDeltaSeconds) 1e+03) "0, 0, 0" "1.000000,1.000000,1.000000"))
  ;[0.15 0.15 0.15 0.5] Checks if we are in position (MoveCharacter keeps being called until we are)
  (if (Utilities|Operators|EqualEqual (Transformation|GetActorLocation (Variables|Default|GetPlayerRef)) (Transformation|GetWorldLocation (select (Variables|/Game/GameBP/Level1/L1_Character.L1_Character_C|GetIsHiding (Variables|Default|GetPlayerRef)) (Variables|Default|GetExitPosition) (Variables|Default|GetHidingPosition))) 0.01)
    ;[0.15 0.15 0.15 0.5] Invalidates both movement timers after we have finished moving
    (Utilities|Time|ClearandInvalidateTimerbyHandle (Variables|Default|GetHideActorTimerHandler))
    (Utilities|Time|ClearandInvalidateTimerbyHandle (stale EventInteract _returnvalue))
    (CallFunction|FinishedMoving)))

(event Custom|FinishedMoving
  (bind _playerref (Variables|Default|GetPlayerRef))
  (bind _playerref_2 (Variables|Default|GetPlayerRef))
  (Default|CallFinishedMovingED)
  ;[0.15 0.15 0.15 0.5] toggles IsHiding bool
  (if (Variables|/Game/GameBP/Level1/L1_Character.L1_Character_C|GetIsHiding _playerref)
    (Variables|/Game/GameBP/Level1/L1_Character.L1_Character_C|SetIsHiding _playerref false)
    ;[0.15 0.15 0.15 0.5] re-enables player movement and collision if we are no longer hiding
    (Collision|SetActorEnableCollision _playerref_2 true)
    (Pawn|Components|CharacterMovement|SetMovementMode (Variables|/Script/Engine.Character|GetCharacterMovement _playerref_2) "MOVE_Walking" 0)
    (Variables|/Game/GameBP/HG_PlayerController.HG_PlayerController_C|SetcanOpenInventory (Variables|Default|GetControllerRef) true)
    (else
      (Variables|/Game/GameBP/Level1/L1_Character.L1_Character_C|SetIsHiding _playerref true))))

(event Custom|RotatePlayer
  ;[0.7843 0.03059 0.02228 0.5] to fix: player rotation when hiding
  (if (Variables|Default|GetShouldRotate)
    (bind _output_get (Variables|Default|SetInitialYawRotation (.yaw (Pawn|GetControlRotation (Variables|Default|GetPlayerRef) :!class /Script/Engine.Pawn))))
    (bind _newtrack_0 (Timeline|Timeline PlayFromStart)
      (:Update
        (Transformation|SetActorRotation (Variables|Default|GetPlayerRef) (Math|Rotator|MakeRotator 0.0 0.0 (Math|Interpolation|Ease "Linear" _newtrack_0 _output_get (.yaw (Transformation|GetWorldRotation (Variables|Default|GetHidingPosition))))))))))

(event EventBeginPlay
  ;[0.15 0.15 0.15 0.5] Creates player reference
  (bind _asl1_character (Utilities|Casting|CastToL1_Character (Game|GetPlayerCharacter 0)))
  (Variables|Default|SetPlayerRef _asl1_character)
  ;[0.15 0.15 0.15 0.5] Creates player controller ref (to access UI)
  (bind _ashg_player_controller (Utilities|Casting|CastToHG_PlayerController (Game|GetPlayerController 0)))
  (Variables|Default|SetControllerRef _ashg_player_controller))

(event EventTick
  (params (DeltaSeconds :type Float%20%28single-precision%29))
  ;[0.15 0.15 0.15 0.5] Contextual Prompt
  (Transformation|SetWorldLocation (Variables|Default|GetContextButtonPromptWidget) (Transformation|GetWorldLocation (Variables|Default|GetSphere)) false false)
  (if (Variables|Default|GetUpdateActor)
    (bind _returnvalue (Collision|LineTraceByChannel (Transformation|GetActorLocation) (Transformation|GetWorldLocation (Variables|/Game/GameBP/Level1/L1_Character.L1_Character_C|GetCamera (Variables|Default|GetPlayerRef))) "TraceTypeQuery1" false 0 "None"))
    (if (not _returnvalue)
      (Rendering|SetVisibility (Variables|Default|GetContextButtonPromptWidget) true false))))

(event EventInteract
  (bind _playerref (Variables|Default|GetPlayerRef))
  (if (Variables|/Game/GameBP/Level1/L1_Character.L1_Character_C|GetIsHiding (Variables|Default|GetPlayerRef))
    (bind _returnvalue (Utilities|Time|SetTimerbyEvent (delegate Custom|MoveCharacter) (Utilities|Time|GetWorldDeltaSeconds) true))
    (else
      (Collision|SetActorEnableCollision _playerref false)
      (Pawn|Components|CharacterMovement|DisableMovement (Variables|/Script/Engine.Character|GetCharacterMovement _playerref))
      (Variables|/Game/GameBP/HG_PlayerController.HG_PlayerController_C|SetcanOpenInventory (Variables|Default|GetControllerRef) false)
      (bind _returnvalue_2 (Utilities|Time|SetTimerbyEvent (delegate Custom|MoveCharacter) (Utilities|Time|GetWorldDeltaSeconds) true))
      (Variables|Default|SetHideActorTimerHandler _returnvalue_2))))

(fn ConstructionScript
  ;[0.15 0.15 0.15 0.5] Allows the distance between the widget and the pickup actor to be adjusted
  (Transformation|SetRelativeLocation (Variables|Default|GetContextButtonPromptWidget) (Transformation|GetWorldLocation (Variables|Default|GetSphere)) false false))
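; Locker hiding spot, a child of a master hide actor, with an animated door the player can also open or shut without hiding.
; Interact swings the door open with a timeline before calling the parent's hide logic and RotatePlayer, alternating ShouldRotate each use.
; The parent's finished-moving dispatcher then triggers the door to close.
; AlternativeInteract toggles the door with sound, and the context prompt shows Open or Close to match.
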(event OnComponentBeginOverlap(Sphere)
  (params (OverlappedComponent :type Primitive%20Component%20Object%20Reference) (OtherActor :type Actor%20Object%20Reference) (OtherComp :type Primitive%20Component%20Object%20Reference) (OtherBodyIndex :type Integer) (bFromSweep :type Boolean) (SweepResult :type Hit%20Result%20Structure%20%28by%20ref%29))
  (bind _contextbuttonpromptwidget (Variables|Default|GetContextButtonPromptWidget))
  (bind _returnvalue (UserInterface|GetUserWidgetObject _contextbuttonpromptwidget))
  ;[0.15 0.15 0.15 0.5] Sets contextual button prompt widget
  (Utilities|Casting|CastToL1_Character OtherActor)
  (bind _asw_context_button_prompt (Utilities|Casting|CastToW_ContextButtonPrompt _returnvalue))
  (Widget|SetVisibility (Variables|/Game/UMG/W_ContextButtonPrompt.W_ContextButtonPrompt_C|GetButtonprompt2 _asw_context_button_prompt) "Visible")
  (bind _asw_context_button_prompt_2 (Utilities|Casting|CastToW_ContextButtonPrompt _returnvalue))
  (Widget|SetVisibility (Variables|/Game/UMG/W_ContextButtonPrompt.W_ContextButtonPrompt_C|GetButtontext2 _asw_context_button_prompt_2) "Visible")
  (bind _asw_context_button_prompt_3 (Utilities|Casting|CastToW_ContextButtonPrompt (UserInterface|GetUserWidgetObject (Variables|Default|GetContextButtonPromptWidget))))
  (Variables|/Script/UMG.TextBlock|SetText (Variables|/Game/UMG/W_ContextButtonPrompt.W_ContextButtonPrompt_C|GetButtonprompt2 _asw_context_button_prompt_3) "T")
  (if (Variables|Default|GetIsClosed)
    (bind _asw_context_button_prompt_4 (Utilities|Casting|CastToW_ContextButtonPrompt (UserInterface|GetUserWidgetObject (Variables|Default|GetContextButtonPromptWidget))))
    (Variables|/Script/UMG.TextBlock|SetText (Variables|/Game/UMG/W_ContextButtonPrompt.W_ContextButtonPrompt_C|GetButtontext2 _asw_context_button_prompt_4) "Open")
    (else
      (bind _asw_context_button_prompt_5 (Utilities|Casting|CastToW_ContextButtonPrompt (UserInterface|GetUserWidgetObject (Variables|Default|GetContextButtonPromptWidget))))
      (Variables|/Script/UMG.TextBlock|SetText (Variables|/Game/UMG/W_ContextButtonPrompt.W_ContextButtonPrompt_C|GetButtontext2 _asw_context_button_prompt_5) "Close"))))

(event Custom|CloseDoor
  (bind _alpha (Timeline|CloseLockerDoor PlayFromStart)
    (:Update
      (Transformation|SetRelativeRotation (Variables|Default|GetDoor) (Math|Rotator|MakeRotator 0.0 0.0 (Math|Float|Lerp 9e+01 0.0 _alpha)) false false))
    (:Finished
      (Variables|Default|SetCanInteract true))))

(event Custom|FinishedMovingED_Event
  ;[0.15 0.15 0.15 0.5] Only allows CloseDoor to be called after finished moving (event dispatch from master hide actor) is complete
  (Utilities|FlowControl|Delay 0.05)
  (CallFunction|CloseDoor))

(event EventBeginPlay
  (|CallParentFunction)
  (EventDispatchers|AssignFinishedMovingED (delegate Custom|FinishedMovingED_Event)))

(event EventAlternativeInteract
  ;[0.15 0.15 0.15 0.5] Opens and closes locker door without hiding on pressing AlternativeInteract
  (if (Variables|Default|GetCanInteract)
    (if (Variables|Default|GetIsClosed)
      (Audio|PlaySound2D "/Game/Sounds/MetalLockerOpeningAudio_Cue.MetalLockerOpeningAudio_Cue" 1.0 1.0 0.0 0 0)
      (Variables|Default|SetCanInteract false)
      (bind _alpha (Timeline|Timeline_0 PlayFromStart)
        (:Update
          (Transformation|SetRelativeRotation (Variables|Default|GetDoor) (Math|Rotator|MakeRotator 0.0 0.0 (Math|Float|Lerp 0.0 9e+01 _alpha)) false false))
        (:Finished
          (Variables|Default|SetCanInteract true)
          (Variables|Default|SetIsClosed false)
          ;[0.15 0.15 0.15 0.5] Updates widget text
          (bind _asw_context_button_prompt (Utilities|Casting|CastToW_ContextButtonPrompt (UserInterface|GetUserWidgetObject (Variables|Default|GetContextButtonPromptWidget))))
          (Variables|/Script/UMG.TextBlock|SetText (Variables|/Game/UMG/W_ContextButtonPrompt.W_ContextButtonPrompt_C|GetButtontext2 _asw_context_button_prompt) "Close")))
      (else
        (Audio|PlaySound2D "/Game/Sounds/MetalLockerShuttingAudio_Cue.MetalLockerShuttingAudio_Cue" 1.0 1.0 0.0 0 0)
        (Variables|Default|SetCanInteract false)
        (bind _alpha_2 (Timeline|Timeline_1 PlayFromStart)
          (:Update
            (Transformation|SetRelativeRotation (Variables|Default|GetDoor) (Math|Rotator|MakeRotator 0.0 0.0 (Math|Float|Lerp 9e+01 0.0 _alpha_2)) false false))
          (:Finished
            (Variables|Default|SetIsClosed true)
            (Variables|Default|SetCanInteract true)
            (bind _asw_context_button_prompt_2 (Utilities|Casting|CastToW_ContextButtonPrompt (UserInterface|GetUserWidgetObject (Variables|Default|GetContextButtonPromptWidget))))
            (Variables|/Script/UMG.TextBlock|SetText (Variables|/Game/UMG/W_ContextButtonPrompt.W_ContextButtonPrompt_C|GetButtontext2 _asw_context_button_prompt_2) "Open")))))))

(event EventInteract
  (Utilities|FlowControl|FlipFlop
    (:A
      (Variables|Default|SetShouldRotate true))
    (:B
      (Variables|Default|SetShouldRotate false)))
  (if (Variables|Default|GetCanInteract)
    (Variables|Default|SetCanInteract false)
    (bind _alpha (Timeline|OpenLockerDoor PlayFromStart)
      (:Update
        (Transformation|SetRelativeRotation (Variables|Default|GetDoor) (Math|Rotator|MakeRotator 0.0 0.0 (Math|Float|Lerp 0.0 9e+01 _alpha)) false false))
      (:Finished
        (Utilities|FlowControl|Delay 0.05)
        ;[0.15 0.15 0.15 0.5] contains all logic in the parent (would be called anyway, but now other functions can be called first on the interact for the locker)
        (|CallParentFunction)
        (CallFunction|RotatePlayer)))))

(fn ConstructionScript
  (|CallParentFunction))
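; Master pickup actor that shows a prompt near the player and adds its item to the player's inventory component.
; Sphere overlap toggles per-tick checks that trace to the player camera, hiding the prompt when blocked and otherwise turning it to face the camera.
; Trace length against PickupDistance switches the prompt icon and actor input.
; The Interact event calls AddItem, destroying the actor when a successful add leaves no remainder.
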(event OnComponentBeginOverlap(Sphere)
  (params (OverlappedComponent :type Primitive%20Component%20Object%20Reference) (OtherActor :type Actor%20Object%20Reference) (OtherComp :type Primitive%20Component%20Object%20Reference) (OtherBodyIndex :type Integer) (bFromSweep :type Boolean) (SweepResult :type Hit%20Result%20Structure%20%28by%20ref%29))
  ;[0.15 0.15 0.15 0.5] When the player enters the sphere, the prompt becomes visible, set updateactor to true
  (bind _asl1_character (Utilities|Casting|CastToL1_Character OtherActor))
  (Variables|Default|SetPlayerRef _asl1_character)
  (Rendering|SetVisibility (Variables|Default|GetPromptWidget) true false)
  (Variables|Default|SetUpdateActor true))

(event OnComponentEndOverlap(Sphere)
  (params (OverlappedComponent :type Primitive%20Component%20Object%20Reference) (OtherActor :type Actor%20Object%20Reference) (OtherComp :type Primitive%20Component%20Object%20Reference) (OtherBodyIndex :type Integer))
  ;[0.15 0.15 0.15 0.5] When the player exits the sphere, the prompt becomes invisible, set update actor to false and disable input on pickup actor
  (Utilities|Casting|CastToL1_Character OtherActor)
  (Rendering|SetVisibility (Variables|Default|GetPromptWidget) false false)
  (Variables|Default|SetUpdateActor false)
  (Input|DisableInput (Game|GetPlayerController 0)))

(event EventInteract
  ;[0.15 0.15 0.15 0.5] Using the interact interface to add items to inventory
  (bind (_success_ _remainder) (Default|AddItem (Variables|/Game/GameBP/Level1/L1_Character.L1_Character_C|GetBPC_Inventory (Variables|Default|GetPlayerRef)) (Variables|Default|GetItem) (Variables|Default|GetAmount)))
  (if _success_
    (if (> _remainder 0)
      (Variables|Default|SetAmount (Variables|Default|GetAmount))
      (else
        (Actor|DestroyActor)))))

(event EventTick
  (params (DeltaSeconds :type Float%20%28single-precision%29))
  (bind _promptwidget (Variables|Default|GetPromptWidget))
  (bind _staticmesh (Variables|Default|GetStaticMesh))
  (bind _returnvalue (Transformation|GetWorldLocation _staticmesh))
  ;[0.15 0.15 0.15 0.5] Keeps widget above mesh
  (Transformation|SetWorldLocation (Variables|Default|GetPromptWidget) (Math|Vector|MakeVector (.x _returnvalue) (.y _returnvalue) (+ (.z _returnvalue) (Variables|Default|GetWidgetDistanceAboveMesh))) false false)
  ;[0.15 0.15 0.15 0.5] If updateactor is true, draw a line trace from the actor to the player camera
  (if (Variables|Default|GetUpdateActor)
    (bind (_outhit _returnvalue_2) (Collision|LineTraceByChannel (Transformation|GetActorLocation) (Transformation|GetWorldLocation (Variables|/Game/GameBP/Level1/L1_Character.L1_Character_C|GetCamera (Variables|Default|GetPlayerRef))) "TraceTypeQuery1" false 0 "ForOneFrame"))
    ;[0.15 0.15 0.15 0.5] If the line trace didn't hit anything in between, set the prompt to visible
    (if (not _returnvalue_2)
      (Rendering|SetVisibility _promptwidget true false)
      ;[0.15 0.15 0.15 0.5] Sets the rotation of the prompt to always face the player camera
      (Transformation|SetWorldRotation (Variables|Default|GetPromptWidget) (Math|Rotator|FindLookatRotation (Transformation|GetWorldLocation (Variables|Default|GetPromptWidget)) (Transformation|GetWorldLocation (Variables|/Game/GameBP/Level1/L1_Character.L1_Character_C|GetCamera (Variables|Default|GetPlayerRef)))) false false)
      ;[0.15 0.15 0.15 0.5] toggles the prompt icon depending on pickup distance
      (Default|TogglePrompt (.AsW%20Pickup%20Prompt (Utilities|Casting|CastToW_PickupPrompt (UserInterface|GetUserWidgetObject (Variables|Default|GetPromptWidget)))) (<= (Math|Vector|VectorLength (- (.TraceStart (Collision|BreakHitResult _outhit)) (.TraceEnd (Collision|BreakHitResult _outhit)))) (Variables|Default|GetPickupDistance)))
      ;[0.15 0.15 0.15 0.5] allows input on pickup actor if we are within pickup distance
      (if (<= (Math|Vector|VectorLength (- (.TraceStart (Collision|BreakHitResult _outhit)) (.TraceEnd (Collision|BreakHitResult _outhit)))) (Variables|Default|GetPickupDistance))
        (Input|EnableInput (Game|GetPlayerController 0))
        (else
          (Input|DisableInput 0)))
      (else
        ;[0.15 0.15 0.15 0.5] if the trace hits something, prevent player input on tthis pickup actor
        (Rendering|SetVisibility _promptwidget false false)
        (Input|DisableInput (Game|GetPlayerController 0))))))

(fn ConstructionScript
  ;[0.15 0.15 0.15 0.5] Allows the distance between the widget and the pickup actor to be adjusted
  (Transformation|SetRelativeLocation (Variables|Default|GetPromptWidget) (Math|Vector|MakeVector 0.0 0.0 (Variables|Default|GetWidgetDistanceAboveMesh)) false false))
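; An interactable door actor that swings open away from the player and closes again on the next interaction.
; On opening, a dot product of the player-to-door direction and the door's forward vector picks which way the 90-degree yaw swing goes.
; A timeline lerps the static mesh's relative rotation, playing from start to open and reversing from end to close, with debug prints.
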(event EventBeginPlay
  (|CallParentFunction) ; This node is disabled and will not be called.\nDrag off pins to build functionality.
)

(event Collision|EventActorBeginOverlap
  (params (OtherActor :type Actor%20Object%20Reference)))

(event EventInteract
  (bind _self self)
  (Development|PrintString "door interacted")
  (if (Variables|Default|GetIsDoorClosed)
    (Variables|Default|SetIsDoorClosed false)
    (Development|PrintString "door is opening")
    (Variables|Default|SetDotProduct (Math|Vector|DotProduct (Math|Vector|Normalize (- (Transformation|GetActorLocation _self) (Transformation|GetActorLocation (Variables|Default|GetPlayerRef)))) (Transformation|GetActorForwardVector _self)))
    (bind _alpha (Timeline|OpenDoor_TL PlayFromStart)
      (:Update
        (Transformation|SetRelativeRotation (Variables|Default|GetStaticMesh_0) (Math|Rotator|MakeRotator 0.0 0.0 (Math|Float|Lerp 0.0 (select (>= (Variables|Default|GetDotProduct) 0.0) 9e+01 -9e+01) _alpha)) false false)))
    (else
      (Variables|Default|SetIsDoorClosed true)
      (Development|PrintString "door is closing")
      (Timeline|OpenDoor_TL ReverseFromEnd))))

(fn ConstructionScript
  (|CallParentFunction))
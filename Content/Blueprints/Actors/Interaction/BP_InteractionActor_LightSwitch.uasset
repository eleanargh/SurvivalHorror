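; An interaction actor that acts as a light switch, toggling a referenced Light actor on and off.
; On BeginPlay it hides the Light's component without a validity check, so the light starts off.
; Interact checks that the Light is valid, then flips the visibility of its LightComponent.
; The construction script only calls the parent implementation.
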(event EventBeginPlay
  (Rendering|SetVisibility (Variables|/Script/Engine.Light|GetLightComponent (Variables|Default|GetLight)) false false))

(event EventInteract
  (bind _light (Variables|Default|GetLight))
  (bind _lightcomponent (Variables|/Script/Engine.Light|GetLightComponent _light))
  ;[1 1 1] Toggles light switch between on and off (if light switch is valid)
  (Utilities|IsValid _light
    (:Is%20Valid
      (if (Variables|/Script/Engine.SceneComponent|GetbVisible _lightcomponent)
        (Rendering|SetVisibility _lightcomponent false false)
        (else
          (Rendering|SetVisibility _lightcomponent true false))))))

(fn ConstructionScript
  (|CallParentFunction))
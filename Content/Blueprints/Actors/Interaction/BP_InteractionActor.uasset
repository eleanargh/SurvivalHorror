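; BP_InteractionActor is an interactable actor that shows a context button prompt when the player's L1_Character is nearby.
; Sphere overlaps toggle the prompt and a flag that enables a per-tick visibility trace to the player camera, which re-shows the prompt when unobstructed.
; The construction script offsets the prompt along Y, but Tick moves it to the sphere's location.
; Interact only prints a placeholder message.
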(event OnComponentBeginOverlap(Sphere)
  (params (OverlappedComponent :type Primitive%20Component%20Object%20Reference) (OtherActor :type Actor%20Object%20Reference) (OtherComp :type Primitive%20Component%20Object%20Reference) (OtherBodyIndex :type Integer) (bFromSweep :type Boolean) (SweepResult :type Hit%20Result%20Structure%20%28by%20ref%29))
  (Utilities|Casting|CastToL1_Character OtherActor)
  (Rendering|SetVisibility (Variables|Default|GetContextButtonPromptWidget) true false)
  (Variables|Default|SetUpdateActor true))

(event OnComponentEndOverlap(Sphere)
  (params (OverlappedComponent :type Primitive%20Component%20Object%20Reference) (OtherActor :type Actor%20Object%20Reference) (OtherComp :type Primitive%20Component%20Object%20Reference) (OtherBodyIndex :type Integer))
  (Utilities|Casting|CastToL1_Character OtherActor)
  (Rendering|SetVisibility (Variables|Default|GetContextButtonPromptWidget) false false)
  (Variables|Default|SetUpdateActor false))

(event EventBeginPlay
  ;[1 1 1] Create player reference
  (bind _asl1_character (Utilities|Casting|CastToL1_Character (Game|GetPlayerCharacter 0)))
  (Variables|Default|SetPlayerRef _asl1_character))

(event EventTick
  (params (DeltaSeconds :type Float%20%28single-precision%29))
  (Transformation|SetWorldLocation (Variables|Default|GetContextButtonPromptWidget) (Transformation|GetWorldLocation (Variables|Default|GetSphere)) false false)
  (if (Variables|Default|GetUpdateActor)
    (bind _returnvalue (Collision|LineTraceByChannel (Transformation|GetActorLocation) (Transformation|GetWorldLocation (Variables|/Game/GameBP/Level1/L1_Character.L1_Character_C|GetCamera (Variables|Default|GetPlayerRef))) "TraceTypeQuery1" false 0 "None"))
    (if (not _returnvalue)
      (Rendering|SetVisibility (Variables|Default|GetContextButtonPromptWidget) true false))))

(event EventInteract
  (Development|PrintString "Hello"))

(fn ConstructionScript
  (Transformation|SetRelativeLocation (Variables|Default|GetContextButtonPromptWidget) (Math|Vector|MakeVector 0.0 (Variables|Default|GetWidgetDistanceInFrontOfActor) 0.0) false false))
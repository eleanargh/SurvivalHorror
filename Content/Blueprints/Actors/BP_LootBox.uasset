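; BP_LootBox is a loot box actor that swings open when its referenced lock is opened.
; On BeginPlay it binds to the lock's LockOpened event dispatcher.
; When that fires, it prints a debug message and plays a timeline that rotates a scene component on roll to open the box.
; Once the timeline finishes, it destroys the lock's dials and the lock actor.
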(event Custom|OpenBoxED_Event
  (bind _lockref (Variables|Default|GetLockRef))
  (Development|PrintString "the box is opening")
  (bind _alpha (Timeline|OpenBoxTL PlayFromStart)
    (:Update
      (Transformation|SetRelativeRotation (Variables|Default|GetScene) (Math|Rotator|MakeRotator (Math|Float|Lerp 0.0 -9e+01 _alpha) 0.0 0.0) false false))
    (:Finished
      (Actor|DestroyActor (Variables|/Game/Blueprints/Actors/BP_Lock.BP_Lock_C|GetDials _lockref))
      (Actor|DestroyActor _lockref))))

(event EventBeginPlay
  (EventDispatchers|BindEventtoLockOpenedED (Variables|Default|GetLockRef) (delegate Custom|OpenBoxED_Event)))

(fn ConstructionScript)
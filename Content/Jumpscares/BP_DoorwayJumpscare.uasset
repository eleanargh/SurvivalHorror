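; BP_DoorwayJumpscare is a jumpscare actor that slides a Quinn skeletal mesh toward an end point.
; While CalledJumpscare is true, Tick moves the mesh at constant InterpSpeed using VInterpToConstant, without sweeping.
; The same Tick chain runs into a short Delay that destroys the actor a few seconds after movement starts.
; Nothing in this graph sets the flag.
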(event EventTick
  (params (DeltaSeconds :type Float%20%28single-precision%29))
  (bind _quinnskelmesh (Variables|Default|GetQuinnSkelMesh))
  (if (Variables|Default|GetcalledJumpscare)
    (Transformation|SetWorldLocation _quinnskelmesh (Math|Interpolation|VInterptoConstant (Transformation|GetWorldLocation _quinnskelmesh) (Transformation|GetWorldLocation (Variables|Default|GetEndPoint)) DeltaSeconds (Variables|Default|GetInterp%20Speed)) false false)
    (Utilities|FlowControl|Delay 3.0)
    (Actor|DestroyActor)))

(fn ConstructionScript)